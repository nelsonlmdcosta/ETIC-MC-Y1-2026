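; Health component that tracks an actor's current and maximum health and handles damage, healing and death.
; On BeginPlay it can optionally start at max health.
; DealDamage and HealDamage only act while health is above zero, clamp the result between zero and max, then fire dispatchers with the amount, current and normalized health.
; DealDamage also fires OnActorDied when health reaches zero, so dead actors cannot be healed.
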(event `self.ReceiveBeginPlay`
  ; Just a quick check to see if we need to set the health or not. Just a nice to have for designers
  (if (`self.ShouldInitializeToMaxHealth`)
    (set `self.CurrentHealth` (`self.MaxHealth`))))

(fn `DealDamage`
  (params (Amount :type "Float (double-precision)"))
  ;[0.15 0 0 0.5] Function Used To Deal Damage To An Entity
  ;; Can't Deal Damage To Something That's Dead
  (if (> (`self.CurrentHealth`) 0.0)
    ;; Clamp The Damage To Keep It Within Min And Max
    (bind _output_get (set `self.CurrentHealth` (`KismetMathLibrary.FClamp` (- (`self.CurrentHealth`) Amount) 0.0 (`self.MaxHealth`))))
    ;; Warn Everyone That's Interesed We Took Damage
    (`self.OnDamageReceived` (`local.Amount`) _output_get (`self.GetNormalizedHealth`))
    ;; Warn Everyone That's Interested We Died
    (if (<= (`self.CurrentHealth`) 0.0)
      (`self.OnActorDied`))))

(fn `GetNormalizedHealth`
  (returns (ReturnValue :type "Float (double-precision)"))
  (return (`KismetMathLibrary.SafeDivide` (`self.CurrentHealth`) (`self.MaxHealth`))))

(fn `HealDamage`
  (params (Amount :type "Float (double-precision)"))
  ;[0.15 0 0 0.5] Function Used For Healing Any Sort Of Damage
  ;; Let's Heal ONLY When We Don't Take Fatal Damage
  (if (> (`self.CurrentHealth`) 0.0)
    ;; Let's Ensure What We Heal Heals Within The Bounds Of The Min And Max
    (set `self.CurrentHealth` (`KismetMathLibrary.FClamp` (+ (`self.CurrentHealth`) Amount) 0.0 (`self.MaxHealth`)))
    ;; Finally Let's Warn Anyone Interested That We've Done The Healing
    (`self.OnDamageHealed` (`local.Amount`) (`self.CurrentHealth`) (`self.GetNormalizedHealth`))))