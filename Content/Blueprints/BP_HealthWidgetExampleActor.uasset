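; Example actor that demonstrates and tests a health component alongside its example UI widget.
; On BeginPlay it binds callbacks to the component's damage, heal and death events, then creates WBP_Example with the component passed in and adds it to the viewport.
; Debug keys heal or damage the component by small random amounts, and the callbacks print colored on-screen messages for each event.
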(event EventBeginPlay
  (Utilities|FlowControl|Sequence
    (:then_0
      (EventDispatchers|BindEventtoOnDamageReceived (Variables|Default|GetBP_HealthComponent) (EventDispatchers|CreateEvent :!event OnDamageReceivedCallback)))
    (:then_1
      (EventDispatchers|BindEventtoOnDamageHealed (Variables|Default|GetBP_HealthComponent) (EventDispatchers|CreateEvent :!event OnDamageHealedCallback)))
    (:then_2
      (EventDispatchers|BindEventtoOnActorDied (Variables|Default|GetBP_HealthComponent) (EventDispatchers|CreateEvent :!event OnActorDiedCallback)))
    (:then_3
      (bind _returnvalue (UserInterface|CreateWidget "/Game/Blueprints/WBP_Example.WBP_Example_C" 0 (Variables|Default|GetBP_HealthComponent)))
      (UserInterface|Viewport|AddtoViewport _returnvalue 0))))

(event Input|KeyboardEvents|DebugKeySubtract
  (params (Key :type Key%20Structure :default "None") (ActionValue :type Input%20Action%20Value%20Structure))
  (:Pressed
    (Default|DealDamage (Variables|Default|GetBP_HealthComponent) (Math|Random|RandomFloatinRange 5.0 1e+01))))

(event Input|KeyboardEvents|DebugKeyAdd
  (params (Key :type Key%20Structure :default "None") (ActionValue :type Input%20Action%20Value%20Structure))
  (:Pressed
    (Default|HealDamage (Variables|Default|GetBP_HealthComponent) (Math|Random|RandomFloatinRange 5.0 1e+01))))

(fn ConstructionScript)

(fn OnDamageReceivedCallback
  (params (Amount :type Float%20%28double-precision%29) (CurrentHealth :type Float%20%28double-precision%29) (NormalziedHealth :type Float%20%28double-precision%29))
  ;[0.15 0.15 0.15 0.5] This gets called when the HealthComponent OnDamageReceivedEvent Is Invoked, We Just Print For Testing Purposes
  (Development|PrintString (Utilities|String|Append "Took Damage: " (Utilities|String|ToString(Float) Amount) " Current Health Is: " (Utilities|String|ToString(Float) CurrentHealth)) true true "(R=1.000000,G=0.017349,B=0.000000,A=1.000000)" 2.0 "42069"))

(fn OnDamageHealedCallback
  (params (Amount :type Float%20%28double-precision%29) (CurrentHealth :type Float%20%28double-precision%29) (NormalizedHealth :type Float%20%28double-precision%29))
  (Development|PrintString (Utilities|String|Append "Healed Damage: " (Utilities|String|ToString(Float) Amount) " Current Health Is: " (Utilities|String|ToString(Float) CurrentHealth)) true true "(R=0.021655,G=1.000000,B=0.000000,A=1.000000)" 2.0 "42069"))

(fn OnActorDiedCallback
  ;[0.15 0.15 0.15 0.5] This gets called when the HealthComponent OnDiedEvent Is Called. We Just Print It Out For Testing Purposes
  (Development|PrintString "Oh Nooooo I Died" true true "(R=0.000000,G=0.114223,B=1.000000,A=1.000000)" 2.0 "42069"))